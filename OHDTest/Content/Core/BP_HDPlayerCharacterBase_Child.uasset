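; Child player character that adds hit feedback, faction death voices and enforcement of the player's weapon selection.
; On spawn it reads BP_WeaponSelectorPlayerState, removes excluded weapons and equips the chosen one after a short delay.
; Excluded items added to the inventory later are destroyed, except on dedicated servers.
; Hit feedback skips zero damage as a friendly-fire fix, and death plays a random sound from the team's faction voice table.
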(event Custom|WeaponSwitch
  (params (Test :type Array%20of%20DF%20Base%20Item%20Class%20References) (NewParam :type DF%20Base%20Item%20Class%20Reference))
  (Development|PrintString "Hello")
  (for _array_element Test
    (Class|DFInventoryComponent|Remove (Variables|Default|GetInventory) (.OutItem (Class|DFInventoryComponent|FindItembyClass (Variables|Default|GetInventory) _array_element)) false)))

(event Custom|CustomEvent_1
  (params (AddedItem :type DF%20Base%20Item%20Object%20Reference))
  (if (not (Networking|IsDedicatedServer))
    (bind _remove_weapons (CallFunction|GetRemovedWeapons))
    (if (Utilities|Array|ContainsItem _remove_weapons (Utilities|GetClass AddedItem))
      (Actor|DestroyActor AddedItem))))

(event EventOnDeath
  (params (KillingDamage :type Float%20%28single-precision%29) (DamageEvent :type Damage%20Event%20Structure%20%28by%20ref%29) (InstigatingPawn :type Pawn%20Object%20Reference) (DamageCauser :type Actor%20Object%20Reference))
  (bind _voices (Variables|Default|GetVoices))
  (bind _returnvalue (Utilities|Array|Length _voices))
  (bind _returnvalue_2 (Math|Random|RandomInteger _returnvalue))
  (bind _output (Utilities|Array|Get(acopy) _voices _returnvalue_2))
  (bind _deathsounds (Utilities|Struct|BreakAICharacterVocalProfile _output))
  ;[1 1 1] Death sound
  (|CallParentFunction KillingDamage DamageEvent InstigatingPawn DamageCauser)
  (bind (_rowname _rowindex _tablerow) (Utilities|ForEachDataTableRow (Utilities|ResolveSoftReference (Utilities|GetClassDefaults (CallFunction|GetHDFactionInfoforTeam (Utilities|Enum|ByteToEnumEHDTeam (Variables|Default|GetTeamNum))))))
    (:LoopBody
      (Utilities|Array|Insert (Variables|Default|GetVoices) _tablerow _rowindex))
    (:Completed
      (Audio|PlaySoundatLocation (Utilities|Array|Get(acopy) _deathsounds (Math|Random|RandomInteger (Utilities|Array|Length _deathsounds))) (Class|DFBlueprintFunctions|GetTargetLocation self 0) "0, 0, 0" 1.0 1.0 0.0 "/HDCore/Characters/Common/Audio/ATT_VocalBarks_CharacterAI.ATT_VocalBarks_CharacterAI" 0 0))))

(event Collision|EventActorBeginOverlap
  (params (OtherActor :type Actor%20Object%20Reference)))

(event EventTick
  (params (DeltaSeconds :type Float%20%28single-precision%29))
  (|CallParentFunction DeltaSeconds) ; This node is disabled and will not be called.\nDrag off pins to build functionality.
)

(event EventPlayHit
  (params (DamageTaken :type Float%20%28single-precision%29) (DamageEvent :type Damage%20Event%20Structure%20%28by%20ref%29) (PawnInstigator :type Pawn%20Object%20Reference) (DamageCauser :type Actor%20Object%20Reference) (bKilled :type Boolean))
  ;[1 0.2031 0.2031] Friendly fire bug fix
  (if (!= DamageTaken 0.0)
    (if (Class|DFBaseCharacter|IsAlive)
      (bind _asdfbase_projectile (Utilities|Casting|CastToDFBaseProjectile DamageCauser)
        (:then
          (CallFunction|HitDamage _asdfbase_projectile))
        (:CastFailed
          (CallFunction|GenericDamageFeedback))))))

(event EventBeginPlay
  (|CallParentFunction)
  (EventDispatchers|BindEventtoOnItemAdded (Variables|Default|GetInventory) (delegate Custom|CustomEvent_1))
  (bind _asbp_weapon_selector_player_state (Utilities|Casting|CastToBP_WeaponSelectorPlayerState (Variables|Default|GetPlayerState)))
  (Variables|/OHDTest/Core/BP_WeaponSelectorPlayerState.BP_WeaponSelectorPlayerState_C|GetWeaponSelected _asbp_weapon_selector_player_state
    (:then
      (CallFunction|WeaponSwitch (Variables|/OHDTest/Core/BP_WeaponSelectorPlayerState.BP_WeaponSelectorPlayerState_C|GetWeaponsToRemove _asbp_weapon_selector_player_state))
      (bind _selectedweapon (CallFunction|GetSeletedWeapon))
      (Utilities|FlowControl|Delay 0.3)
      (if (Utilities|IsValid (.OutItem (Class|DFInventoryComponent|FindItembyClass (Variables|Default|GetInventory) _selectedweapon)))
        (Class|DFBaseCharacter|EquipItem (.OutItem (Class|DFInventoryComponent|FindItembyClass (Variables|Default|GetInventory) _selectedweapon)))))
    (:else)))

(fn ConstructionScript
  (|CallParentFunction))

(fn GetMostValidLoadout
  (return (|CallParentFunction)))

(fn GetRemovedWeapons
  (bind _asbp_weapon_selector_player_state (Utilities|Casting|CastToBP_WeaponSelectorPlayerState (Variables|Default|GetPlayerState)))
  (return (Variables|/OHDTest/Core/BP_WeaponSelectorPlayerState.BP_WeaponSelectorPlayerState_C|GetWeaponsToRemove _asbp_weapon_selector_player_state)))

(fn GetSeletedWeapon
  (bind _asbp_weapon_selector_player_state (Utilities|Casting|CastToBP_WeaponSelectorPlayerState (Variables|Default|GetPlayerState)))
  (return (Variables|/OHDTest/Core/BP_WeaponSelectorPlayerState.BP_WeaponSelectorPlayerState_C|GetWeaponSelected _asbp_weapon_selector_player_state)))