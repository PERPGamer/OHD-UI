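; BP_HDPlayerControllerBase_Edit is a player controller that manages the edited deploy menu, wounded screen and death camera.
; It creates the edited widgets, preloads the deploy menu, and toggles it through the menu manager alongside HUD visibility and scoreboard unloading.
; A Force flag overrides victory-screen precedence and initial-spawn blocking, and enables UI-only input.
; On character death, it re-targets the victim controller's view to the pawn after a short delay.
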(event EventTick
  (params (DeltaSeconds :type Float%20%28single-precision%29)))

(event EventCharacterDeath
  (params (VictimPawn :type Pawn%20Object%20Reference) (VictimController :type Controller%20Object%20Reference) (KillingDamage :type Float%20%28single-precision%29) (DamageEvent :type Damage%20Event%20Structure%20%28by%20ref%29) (InstigatingPawn :type Pawn%20Object%20Reference) (DamageCauser :type Actor%20Object%20Reference))
  ;[1 1 1] Allows camera to stay active while dying
  (|CallParentFunction VictimPawn VictimController KillingDamage DamageEvent InstigatingPawn DamageCauser)
  (bind _ashdplayer_controller (Utilities|Casting|CastToHDPlayerController VictimController))
  (Utilities|FlowControl|Delay 0.1)
  (Game|Player|SetViewTargetwithBlend _ashdplayer_controller VictimPawn 0.0 "VTBlend_Linear" 0.0 false))

(fn ConstructionScript
  (|CallParentFunction))

(fn LoadDeathScreen
  (Utilities|IsValid (Variables|Default|GetDeathScreen)
    (:Is%20Not%20Valid
      (bind _returnvalue (UserInterface|CreateWidget "/OHDTest/UI/Interaction/WBP_WoundedScreen_Edit.WBP_WoundedScreen_Edit_C" self))
      (Variables|Default|SetDeathScreen _returnvalue))))

(fn DeployMenuToggle
  (params (bShowMenu :type Boolean) (bForce :type Boolean))
  (bind _deploymenu (Variables|Default|GetDeployMenu)
    (:then
      (if bShowMenu
        (if (Math|Boolean|ANDBoolean (not (UserInterface|Viewport|IsinViewport _deploymenu)) (Variables|/HDCore/UI/DeployMenu/WBP_DeployMenu.WBP_DeployMenu_C|GetbDonePreloading _deploymenu) (or (not (CallFunction|IsVictoryMenuShown)) bForce))
          (Class|DFMenuManager|ActivateMenu (Class|DFMenuManagerBlueprintFunctions|GetMenuManager) (Variables|Default|GetDeployMenu) "Exclusive" true bForce)
          (bind _output_get (Variables|Default|SetbWantsToOpenDeployMenu bShowMenu :!label _label))
          (bind _output_get_2 (Variables|Default|SetbDeployMenuShown _output_get))
          (if _output_get_2
            (CallFunction|HideHUD)
            (Class|HDGameInstance|UnloadScoreboardMenu (.AsHDGame%20Instance (Utilities|Casting|CastToHDGameInstance (Game|GetGameInstance))))
            (else
              (CallFunction|ShowHUD))))
        (elif (and (not (Variables|/Script/DonkehFrameworkUI.DFBaseMenu|GetbMenuPopped (Variables|Default|GetDeployMenu))) (or (not (Variables|Default|GetbInitialSpawn)) bForce))
          (Class|DFBaseMenu|RemovefromMenuStack (Variables|Default|GetDeployMenu))
          (goto _label))))
    (:else)))

(fn LoadDeployMenu
  (Utilities|IsValid (Variables|Default|GetDeployMenu)
    (:Is%20Not%20Valid
      (bind _returnvalue (UserInterface|CreateWidget "/OHDTest/UI/DeployMenu/WBP_DeployMenu_Edited.WBP_DeployMenu_Edited_C" self 0 0))
      (bind _output_get (Variables|Default|SetDeployMenu _returnvalue)) ; Store widget reference
      (EventDispatchers|BindEventtoOnPreloadFinished _output_get (EventDispatchers|CreateEvent :!event OnDeployMenuPreloadFinished))
      (Default|PreloadContent (Variables|Default|GetDeployMenu)))))

(fn LoadandActivateDeployMenu
  (bind _returnvalue (Class|DFMenuManagerBlueprintFunctions|CreateandActivate "/OHDTest/UI/DeployMenu/WBP_DeployMenu_Edited.WBP_DeployMenu_Edited_C" self "Exclusive" true false))
  (Variables|Default|SetDeployMenu _returnvalue) ; Store widget reference
  (Variables|Default|SetbDeployMenuShown true)
  (CallFunction|HideHUD)
  (Class|HDGameInstance|UnloadScoreboardMenu (.AsHDGame%20Instance (Utilities|Casting|CastToHDGameInstance (Game|GetGameInstance)))))