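; Player controller that shows and updates a vehicle seat HUD while the player is in a vehicle.
; As a workaround for no vehicle-entry event, Tick polls IsInVehicle, runs HUD setup once via a resettable DoOnce, and refreshes seats every frame.
; Setup reveals and populates the widget already inside the HUD container.
; Seat change requests also refresh it, and leaving the vehicle or requesting exit hides it.
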(event Custom|RemoveHud
  (CallFunction|RemoveVehicleHUD))

(event EventBeginPlay
  (|CallParentFunction))

(event EventTick
  (params (DeltaSeconds :type Float%20%28single-precision%29))
  ;[1 0.2135 0.2135] Work around since no current way of checking if a player gets into a vehicle outside the vehicle base blueprint
  (|CallParentFunction DeltaSeconds)
  (if (Class|HDPlayerController|IsinVehicle)
    (Utilities|FlowControl|Sequence
      (:then_0
        (Utilities|FlowControl|DoOnce false :!label _label
          (:Completed
            (CallFunction|SetupVehicleHUD))))
      (:then_1
        (CallFunction|ChangeSeats)))
    (else
      (CallFunction|RemoveHud)
      (goto _label Reset))))

(event EventRequestSeatChange
  (params (Seat :type Integer))
  (|CallParentFunction Seat)
  (CallFunction|ChangeSeats))

(event EventServerRequestExitVehicle
  (params (Vehicle :type Arc%20Base%20Vehicle%20Object%20Reference))
  (CallFunction|RemoveHud)
  (|CallParentFunction Vehicle))

(fn ConstructionScript
  (|CallParentFunction))

(fn SetupVehicleHUD
  (bind _returnvalue (HUD|GetHUD))
  (bind _asbp_hdhud_vehicle_hudtest (Utilities|Casting|CastToBP_HDHUD_VehicleHUDTest _returnvalue))
  (Variables|/Script/Engine.HUD|SetbShowHUD _returnvalue true)
  (Widget|SetVisibility (Variables|/VehicleHUD/UI/HUD/WBP_HUDProtype.WBP_HUDProtype_C|GetVehicleHUD (.AsWBP%20HUDProtype (Utilities|Casting|CastToWBP_HUDProtype (Variables|/HDCore/Core/BP_HDHUDBase.BP_HDHUDBase_C|GetHUDContainerUW _asbp_hdhud_vehicle_hudtest)))) "Visible")
  (bind _output_get (Variables|Default|SetVehicleHUD (Variables|/VehicleHUD/UI/HUD/WBP_HUDProtype.WBP_HUDProtype_C|GetVehicleHUD (.AsWBP%20HUDProtype (Utilities|Casting|CastToWBP_HUDProtype (Variables|/HDCore/Core/BP_HDHUDBase.BP_HDHUDBase_C|GetHUDContainerUW _asbp_hdhud_vehicle_hudtest))))))
  (Default|SetUpPlayers _output_get))

(fn RemoveVehicleHUD
  (bind _vehiclehud (Variables|Default|GetVehicleHUD)
    (:then
      (Widget|SetVisibility _vehiclehud "Hidden")
      (Default|OnVehicleExit _vehiclehud))
    (:else)))

(fn ChangeSeats
  (bind _vehiclehud (Variables|Default|GetVehicleHUD)
    (:then
      (Default|SeatChange _vehiclehud))
    (:else)))